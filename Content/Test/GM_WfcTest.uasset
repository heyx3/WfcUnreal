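; Test game mode that runs a Wave Function Collapse generator on a 3D grid from a tileset.
; BeginPlay seeds and starts it; Tick steps it several times per frame, printing progress until completion, tick limit or manual stop.
; Results spawn as static mesh actors; unset cells hotter than median temperature get failed-tile markers shaded green to red.
; InitializeGrid is an empty function called after startup.
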(event Custom|Stop%20Generation
  (bind _tileset (Variables|Default|GetTileset))
  (bind _grid_size (Variables|Default|GetGrid%20Size))
  (bind (_x _y _z) (Utilities|Struct|BreakIntVector _grid_size))
  (bind _tilelength (Variables|/Script/WFCpp2UnrealRuntime.WfcTileset|GetTileLength _tileset))
  (if (Class|WfcGenerator|IsRunning (Variables|Default|GetGenerator))
    (Class|WfcGenerator|Stop (Variables|Default|GetGenerator))
    (bind (_min _max _mean _median) (Class|WfcGenerator|GetTemperatureData (Variables|Default|GetGenerator)))
    (for _index (range 0 (- _x 1))
      (for _index_2 (range 0 (- _y 1))
        (for _index_3 (range 0 (- _z 1))
          (if (.IsSet (Utilities|Struct|BreakWfcCellStatus (Class|WfcGenerator|GetCell (Variables|Default|GetGenerator) (Utilities|Struct|MakeIntVector _index _index_2 _index_3))))
            (CallFunction|SpawnTile (.tileid (.IfSet (Utilities|Struct|BreakWfcCellStatus (Class|WfcGenerator|GetCell (Variables|Default|GetGenerator) (Utilities|Struct|MakeIntVector _index _index_2 _index_3))))) (.tilegamedata (.IfSet (Utilities|Struct|BreakWfcCellStatus (Class|WfcGenerator|GetCell (Variables|Default|GetGenerator) (Utilities|Struct|MakeIntVector _index _index_2 _index_3))))) (Math|Transform|MakeTransform (+ (.Location (Math|Transform|BreakTransform (Class|WfcUtils|WfctoFTransform (.tilepermutation (.IfSet (Utilities|Struct|BreakWfcCellStatus (Class|WfcGenerator|GetCell (Variables|Default|GetGenerator) (Utilities|Struct|MakeIntVector _index _index_2 _index_3)))))))) (* (Math|Conversions|ToVector(Float) (Utilities|Struct|MakeIntVector _index _index_2 _index_3)) _tilelength)) (.Rotation (Math|Transform|BreakTransform (Class|WfcUtils|WfctoFTransform (.tilepermutation (.IfSet (Utilities|Struct|BreakWfcCellStatus (Class|WfcGenerator|GetCell (Variables|Default|GetGenerator) (Utilities|Struct|MakeIntVector _index _index_2 _index_3)))))))) (.Scale (Math|Transform|BreakTransform (Class|WfcUtils|WfctoFTransform (.tilepermutation (.IfSet (Utilities|Struct|BreakWfcCellStatus (Class|WfcGenerator|GetCell (Variables|Default|GetGenerator) (Utilities|Struct|MakeIntVector _index _index_2 _index_3))))))))))
            (elif (< _median (.Temperature (Utilities|Struct|BreakWfcCellStatus (Class|WfcGenerator|GetCell (Variables|Default|GetGenerator) (Utilities|Struct|MakeIntVector _index _index_2 _index_3)))))
              (Game|SpawnActorfromClass "/WFCpp2/Test/A_WFCTest_FailedTile.A_WFCTest_FailedTile_C" (Math|Transform|MakeTransform (+ (.Location (Math|Transform|BreakTransform (Class|WfcUtils|WfctoFTransform (.tilepermutation (.IfSet (Utilities|Struct|BreakWfcCellStatus (Class|WfcGenerator|GetCell (Variables|Default|GetGenerator) (Utilities|Struct|MakeIntVector _index _index_2 _index_3)))))))) (* (Math|Conversions|ToVector(Float) (Utilities|Struct|MakeIntVector _index _index_2 _index_3)) _tilelength)) (.Rotation (Math|Transform|BreakTransform (Class|WfcUtils|WfctoFTransform (.tilepermutation (.IfSet (Utilities|Struct|BreakWfcCellStatus (Class|WfcGenerator|GetCell (Variables|Default|GetGenerator) (Utilities|Struct|MakeIntVector _index _index_2 _index_3)))))))) (.Scale (Math|Transform|BreakTransform (Class|WfcUtils|WfctoFTransform (.tilepermutation (.IfSet (Utilities|Struct|BreakWfcCellStatus (Class|WfcGenerator|GetCell (Variables|Default|GetGenerator) (Utilities|Struct|MakeIntVector _index _index_2 _index_3))))))))) "Undefined" "MultiplyWithRoot" 0 _tilelength "0.000000,0.000000,0.000000" (Math|Color|Lerp(LinearColor) "(R=0.000000,G=0.166667,B=0.011710,A=1.000000)" "(R=1.000000,G=0.000000,B=0.000000,A=1.000000)" (Utilities|InverseLerpD _median _max (.Temperature (Utilities|Struct|BreakWfcCellStatus (Class|WfcGenerator|GetCell (Variables|Default|GetGenerator) (Utilities|Struct|MakeIntVector _index _index_2 _index_3)))))) 0)
              (Development|PrintString "Hello"))))))))

(event EventBeginPlay
  (bind _periodic_ (Variables|Default|GetPeriodic?))
  (Variables|Default|SetSeed%20%28if%20not%20random%29 (Math|Integer|SelectInt (Math|Random|RandomInteger 1999999999) (Variables|Default|GetSeed%20%28if%20not%20random%29) (Variables|Default|GetRandom%20Seed?)))
  (bind _returnvalue (Game|ConstructObjectfromClass "/Script/WFCpp2UnrealRuntime.WfcGenerator"))
  (bind _output_get (Variables|Default|SetGenerator _returnvalue))
  (Class|WfcGenerator|Start _output_get (Variables|Default|GetTileset) (Variables|Default|GetGrid%20Size) (Variables|Default|GetSeed%20%28if%20not%20random%29) (Variables|Default|GetTemperature%20Clear%20Growth%20Rate%20T) (Variables|Default|GetFuzziness) (Variables|Default|GetMax%20Unwinding) _periodic_ _periodic_ _periodic_)
  (CallFunction|InitializeGrid))

(event EventTick
  (params (DeltaSeconds :type Float%20%28single-precision%29))
  (bind _tileset (Variables|Default|GetTileset))
  (bind _grid_size (Variables|Default|GetGrid%20Size))
  (bind _grid_size_2 (Variables|Default|GetGrid%20Size))
  (bind _generator (Variables|Default|GetGenerator))
  (bind _grid_size_3 (Variables|Default|GetGrid%20Size))
  (bind (_x _y _z) (Utilities|Struct|BreakIntVector _grid_size_3))
  (bind (_x_2 _y_2 _z_2) (Utilities|Struct|BreakIntVector _grid_size))
  (bind (_x_3 _y_3 _z_3) (Utilities|Struct|BreakIntVector _grid_size_2))
  (bind _tilelength (Variables|/Script/WFCpp2UnrealRuntime.WfcTileset|GetTileLength _tileset))
  (|CallParentFunction DeltaSeconds)
  (for _index (range 1 (Variables|Default|GetTicks%20Per%20Tick))
    (if (Class|WfcGenerator|IsRunning _generator)
      (Utilities|FlowControl|Sequence
        (:then_0
          (Class|WfcGenerator|Tick _generator)
          (|IsStillRunning?
            (:Finished%20Running
              (Class|WfcGenerator|Stop (Variables|Default|GetGenerator))
              (bind (_min _max _mean _median) (Class|WfcGenerator|GetTemperatureData (Variables|Default|GetGenerator) :!label _label))
              (for _index_2 (range 0 (- _x 1))
                (for _index_3 (range 0 (- _y 1))
                  (for _index_4 (range 0 (- _z 1))
                    (if (.IsSet (Utilities|Struct|BreakWfcCellStatus (Class|WfcGenerator|GetCell (Variables|Default|GetGenerator) (Utilities|Struct|MakeIntVector _index_2 _index_3 _index_4))))
                      (CallFunction|SpawnTile (.tileid (.IfSet (Utilities|Struct|BreakWfcCellStatus (Class|WfcGenerator|GetCell (Variables|Default|GetGenerator) (Utilities|Struct|MakeIntVector _index_2 _index_3 _index_4))))) (.tilegamedata (.IfSet (Utilities|Struct|BreakWfcCellStatus (Class|WfcGenerator|GetCell (Variables|Default|GetGenerator) (Utilities|Struct|MakeIntVector _index_2 _index_3 _index_4))))) (Math|Transform|MakeTransform (+ (.Location (Math|Transform|BreakTransform (Class|WfcUtils|WfctoFTransform (.tilepermutation (.IfSet (Utilities|Struct|BreakWfcCellStatus (Class|WfcGenerator|GetCell (Variables|Default|GetGenerator) (Utilities|Struct|MakeIntVector _index_2 _index_3 _index_4)))))))) (* (Math|Conversions|ToVector(Float) (Utilities|Struct|MakeIntVector _index_2 _index_3 _index_4)) _tilelength)) (.Rotation (Math|Transform|BreakTransform (Class|WfcUtils|WfctoFTransform (.tilepermutation (.IfSet (Utilities|Struct|BreakWfcCellStatus (Class|WfcGenerator|GetCell (Variables|Default|GetGenerator) (Utilities|Struct|MakeIntVector _index_2 _index_3 _index_4)))))))) (.Scale (Math|Transform|BreakTransform (Class|WfcUtils|WfctoFTransform (.tilepermutation (.IfSet (Utilities|Struct|BreakWfcCellStatus (Class|WfcGenerator|GetCell (Variables|Default|GetGenerator) (Utilities|Struct|MakeIntVector _index_2 _index_3 _index_4))))))))))
                      (elif (< _median (.Temperature (Utilities|Struct|BreakWfcCellStatus (Class|WfcGenerator|GetCell (Variables|Default|GetGenerator) (Utilities|Struct|MakeIntVector _index_2 _index_3 _index_4)))))
                        (Game|SpawnActorfromClass "/WFCpp2/Test/A_WFCTest_FailedTile.A_WFCTest_FailedTile_C" (Math|Transform|MakeTransform (+ (.Location (Math|Transform|BreakTransform (Class|WfcUtils|WfctoFTransform (.tilepermutation (.IfSet (Utilities|Struct|BreakWfcCellStatus (Class|WfcGenerator|GetCell (Variables|Default|GetGenerator) (Utilities|Struct|MakeIntVector _index_2 _index_3 _index_4)))))))) (* (Math|Conversions|ToVector(Float) (Utilities|Struct|MakeIntVector _index_2 _index_3 _index_4)) _tilelength)) (.Rotation (Math|Transform|BreakTransform (Class|WfcUtils|WfctoFTransform (.tilepermutation (.IfSet (Utilities|Struct|BreakWfcCellStatus (Class|WfcGenerator|GetCell (Variables|Default|GetGenerator) (Utilities|Struct|MakeIntVector _index_2 _index_3 _index_4)))))))) (.Scale (Math|Transform|BreakTransform (Class|WfcUtils|WfctoFTransform (.tilepermutation (.IfSet (Utilities|Struct|BreakWfcCellStatus (Class|WfcGenerator|GetCell (Variables|Default|GetGenerator) (Utilities|Struct|MakeIntVector _index_2 _index_3 _index_4))))))))) "Undefined" "MultiplyWithRoot" 0 _tilelength "0.000000,0.000000,0.000000" (Math|Color|Lerp(LinearColor) "(R=0.000000,G=0.166667,B=0.011710,A=1.000000)" "(R=1.000000,G=0.000000,B=0.000000,A=1.000000)" (Utilities|InverseLerpD _median _max (.Temperature (Utilities|Struct|BreakWfcCellStatus (Class|WfcGenerator|GetCell (Variables|Default|GetGenerator) (Utilities|Struct|MakeIntVector _index_2 _index_3 _index_4)))))) 0)
                        (Development|PrintString "Hello")))))))))
        (:then_1
          (Development|PrintString (Utilities|String|Append (Utilities|String|ToString(Integer) (Class|WfcGenerator|GetTickCount _generator)) " / " (Utilities|String|ToString(Integer) (* _x_3 _y_3 _z_3)) " == " (Utilities|String|ToString(Float) (Class|WfcGenerator|GetProgress _generator))) true true "(R=0.000000,G=1.000000,B=0.266667,A=1.000000)" 999.0 "WFCPP_PROGRESS_TEST"))
        (:then_2
          (if (and (> (Variables|Default|GetThreshold%20relative%20tick%20count%20to%20give%20up) 0.0) (> (Math|Conversions|ToFloat(Integer) (Class|WfcGenerator|GetTickCount (Variables|Default|GetGenerator))) (* (Variables|Default|GetThreshold%20relative%20tick%20count%20to%20give%20up) _x_2 _y_2 _z_2)))
            (Development|PrintString (Utilities|String|Append "Gave up on iteration " (Utilities|String|ToString(Integer) (Class|WfcGenerator|GetTickCount _generator))) true true "(R=1.000000,G=0.850459,B=0.000000,A=1.000000)" 9999.0 "WFC_TEST_GAVE_UP")
            (Class|WfcGenerator|Stop (Variables|Default|GetGenerator))
            (goto _label)))))))

(fn ConstructionScript)

(fn SpawnTile
  (params (Tile%20ID :type Integer) (Tile%20Data :type Object%20Object%20Reference) (Spawn%20Transform :type Transform))
  (bind _aswfc_tile_game_data_static_mesh (Utilities|Casting|CastToWfcTileGameData_StaticMesh Tile%20Data))
  (bind _returnvalue (Game|SpawnActorfromClass "/Script/Engine.StaticMeshActor" Spawn%20Transform "AlwaysSpawn" "MultiplyWithRoot" 0 0))
  (Transformation|SetMobility _returnvalue "Movable")
  (Components|StaticMesh|SetStaticMesh (Variables|/Script/Engine.StaticMeshActor|GetStaticMeshComponent _returnvalue) (Variables|/Script/WFCpp2UnrealRuntime.WfcTileGameData_StaticMesh|GetMesh _aswfc_tile_game_data_static_mesh))
  (return _returnvalue))

(fn InitializeGrid)

(fn InverseLerp
  (params (A :type Float%20%28double-precision%29) (B :type Float%20%28double-precision%29) (X :type Float%20%28double-precision%29))
  (return 0.0))